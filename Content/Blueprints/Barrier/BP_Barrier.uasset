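; BP_Barrier is a breakable barrier that is destroyed when the turtle attacks it.
; Its BarrierHitbox begin overlap filters for the TurtleAttackHitbox component tag, then sets an overlap flag and caches the BPC_Turtle.
; Tick polls that turtle's IsAttacking state during overlap and destroys the barrier when true.
; Any end overlap on the hitbox clears both reference and flag, without a tag check.
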(event OnComponentBeginOverlap(BarrierHitbox)
  (params (OverlappedComponent :type Primitive%20Component%20Object%20Reference) (OtherActor :type Actor%20Object%20Reference) (OtherComp :type Primitive%20Component%20Object%20Reference) (OtherBodyIndex :type Integer) (bFromSweep :type Boolean) (SweepResult :type Hit%20Result%20Structure%20%28by%20ref%29))
  (if (Components|ComponentHasTag OtherComp "TurtleAttackHitbox")
    (Variables|Default|SetTurtleIsOverlapping true)
    (bind _asbpc_turtle (Utilities|Casting|CastToBPC_Turtle OtherActor))
    (Variables|Default|SetTurtle _asbpc_turtle)))

(event OnComponentEndOverlap(BarrierHitbox)
  (params (OverlappedComponent :type Primitive%20Component%20Object%20Reference) (OtherActor :type Actor%20Object%20Reference) (OtherComp :type Primitive%20Component%20Object%20Reference) (OtherBodyIndex :type Integer))
  (Variables|Default|SetTurtle 0)
  (Variables|Default|SetTurtleIsOverlapping false))

(event EventBeginPlay)

(event Collision|EventActorBeginOverlap
  (params (OtherActor :type Actor%20Object%20Reference)))

(event EventTick
  (params (DeltaSeconds :type Float%20%28single-precision%29))
  (bind _turtle (Variables|Default|GetTurtle))
  (if (!= _turtle 0)
    (if (and (Variables|Default|GetTurtleIsOverlapping) (Variables|/Game/Blueprints/Turtle/BPC_Turtle.BPC_Turtle_C|GetIsAttacking _turtle))
      (Actor|DestroyActor))))

(event Collision|EventActorEndOverlap
  (params (OtherActor :type Actor%20Object%20Reference)))

(fn ConstructionScript)