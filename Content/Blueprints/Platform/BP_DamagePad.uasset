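; Damage pad that knocks the player turtle (BPC_Turtle) back and costs it a point when it overlaps the pad's hitbox.
; The sign of the turtle's last X velocity picks an opposing horizontal launch with upward lift, or a purely vertical launch when it is zero.
; Each branch then decrements any positive score and prints the result.
; The construction script hard-sets both launch speeds.
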(event OnComponentBeginOverlap(BoostPadHitbox)
  (params (OverlappedComponent :type Primitive%20Component%20Object%20Reference) (OtherActor :type Actor%20Object%20Reference) (OtherComp :type Primitive%20Component%20Object%20Reference) (OtherBodyIndex :type Integer) (bFromSweep :type Boolean) (SweepResult :type Hit%20Result%20Structure%20%28by%20ref%29))
  (bind _asbpc_turtle (Utilities|Casting|CastToBPC_Turtle OtherActor))
  (if (< (.x (Pawn|Components|CharacterMovement|GetLastUpdateVelocity (Variables|/Script/Engine.Character|GetCharacterMovement _asbpc_turtle))) 0.0)
    (Character|LaunchCharacter _asbpc_turtle (Math|Vector|MakeVector (Variables|Default|GetHorizontalLaunchSpeed) 0.0 (Variables|Default|GetVerticalLaucnhSpeed)) true true)
    (if (> (Variables|/Game/Blueprints/Turtle/BPC_Turtle.BPC_Turtle_C|GetScore _asbpc_turtle) 0) :!label _label
      (bind _new_score (Default|AddtoScore _asbpc_turtle -1))
      (Development|PrintString (Utilities|String|ToString(Integer) _new_score)))
    (elif (> (.x (Pawn|Components|CharacterMovement|GetLastUpdateVelocity (Variables|/Script/Engine.Character|GetCharacterMovement _asbpc_turtle))) 0.0)
      (Character|LaunchCharacter _asbpc_turtle (Math|Vector|MakeVector (* (Variables|Default|GetHorizontalLaunchSpeed) -1.0) 0.0 (Variables|Default|GetVerticalLaucnhSpeed)) true true)
      (goto _label)
      (elif (== (.x (Pawn|Components|CharacterMovement|GetLastUpdateVelocity (Variables|/Script/Engine.Character|GetCharacterMovement _asbpc_turtle))) 0.0)
        (Character|LaunchCharacter _asbpc_turtle (Math|Vector|MakeVector 0.0 0.0 (Variables|Default|GetVerticalLaucnhSpeed)) false true)
        (goto _label)))))

(event EventBeginPlay)

(event Collision|EventActorBeginOverlap
  (params (OtherActor :type Actor%20Object%20Reference)))

(event EventTick
  (params (DeltaSeconds :type Float%20%28single-precision%29)))

(fn ConstructionScript
  (Variables|Default|SetVerticalLaucnhSpeed 3e+02)
  (Variables|Default|SetHorizontalLaunchSpeed 3e+02))